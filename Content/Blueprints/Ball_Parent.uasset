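; Parent Blueprint for balls in a cue game that can return to their starting position on restart.
; On BeginPlay each ball adds itself to the player Cue_Character's Balls array and binds RestartBall to that character's restart event.
; It also caches its spawn location, and RestartBall teleports it back there without sweeping.
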(event `self.ReceiveBeginPlay`
  (bind _ascue_character (cast `/Game/Cue_Character` (`GameplayStatics.GetPlayerPawn` 0)))
  (`KismetArrayLibrary.Array_Add` (`/Game/Cue_Character.Balls` _ascue_character) self)
  (add `/Game/Cue_Character.Restart` _ascue_character (delegate `Restart Ball`))
  (set `self.Initial Location` (`self.K2_GetActorLocation`)))

(event `Restart Ball`
  (`self.K2_SetActorLocation` (`self.Initial Location`) false true))

(fn `UserConstructionScript`)