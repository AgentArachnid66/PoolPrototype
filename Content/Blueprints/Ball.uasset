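; Ball Blueprint for a cue-and-pocket game that awards score when it enters a pocket.
; On overlapping a Pocket, it adds its Points to the Score of the player's Cue_Character and hides its Sphere mesh rather than destroying the actor.
; RestartBall calls the parent implementation, then makes the Sphere visible again.
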(event `self.ReceiveBeginPlay`
  (`parent.ReceiveBeginPlay`))

(event `self.ReceiveActorBeginOverlap`
  (params (OtherActor :type "Actor Object Reference"))
  (`parent.ReceiveActorBeginOverlap` OtherActor)
  (cast `/Game/Blueprints/Pocket` OtherActor)
  (bind _ascue_character (cast `/Game/Cue_Character` (`GameplayStatics.GetPlayerPawn` 0)))
  (set `/Game/Cue_Character.Score` (+ (`/Game/Cue_Character.Score` _ascue_character) (`self.Points`)) _ascue_character)
  (`SceneComponent.SetVisibility` (`self.Sphere`) false false))

(event `self.Restart Ball`
  (`parent.Restart Ball`)
  (`SceneComponent.SetVisibility` (`self.Sphere`) true false))

(fn `UserConstructionScript`
  (`parent.UserConstructionScript`))